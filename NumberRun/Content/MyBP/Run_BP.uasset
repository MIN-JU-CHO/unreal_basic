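; Runner actor Blueprint for a race, moving along its local Y axis at a random speed.
; Tick offsets it by a random step scaled by DeltaMoveY until IsStopLocal is set; CE_SetDeltaMoveY supplies that multiplier to start it.
; CE_setResult, noted as the trigger-box collision response, sets the stop flag and raises the runner by its rank, like a podium.
; CE_High is a similar height offset marked as trash.
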(event `self.ReceiveTick`
  (params (DeltaSeconds :type "Float (single-precision)"))
  ;[1 1 1] Running with random speed
  ; (at first Delta=0, so no move)
  ; (if Delta=1 from CE call -> start move)
  (if (not (`self.isStop_Local`))
    (`self.K2_AddActorLocalOffset` (`KismetMathLibrary.MakeVector` 0.0 (* (`KismetMathLibrary.RandomFloatInRange` 0.1 3.0) (`self.Delta_Move_Y`))))))

(event `CE_setResult`
  (params (isstop :type Boolean) (fl_high :type Integer))
  ;[1 1 1] if collision with triggerbox :
  ; set stop and move high as much as its each rank
  (set `self.isStop_Local` isstop)
  (`self.K2_AddActorLocalOffset` (`KismetMathLibrary.MakeVector` 0.0 0.0 (* (`KismetMathLibrary.Conv_IntToDouble` (- 4 fl_high)) 100.0))))

(event `CE_High`
  (params (fl_high :type Integer))
  ;[1 1 1] trash
  (`self.K2_AddActorLocalOffset` (`KismetMathLibrary.MakeVector` 0.0 0.0 (* (`KismetMathLibrary.Conv_IntToDouble` (- 4 fl_high)) 50.0))))

(event `CE_SetDeltaMoveY`
  (params (Delta :type "Float (double-precision)"))
  ;[1 1 1] start runners
  (set `self.Delta_Move_Y` Delta))

(fn `UserConstructionScript`)