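; BP_GameManager is a trigger-box actor that recycles road pieces by passing them to their road controllers for respawning.
; On box overlap it prints the other actor's name, then casts it to center, left or right road types.
; A match calls ReSpawnActor on the corresponding center, left or right controller reference.
; The construction script sets the box's Y extent from the BoxCollisionHeight variable, keeping X and Z.
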(event `self.BoxCollision.OnComponentBeginOverlap`
  (params (OverlappedComponent :type "PrimitiveComponent Object Reference") (OtherActor :type "Actor Object Reference") (OtherComp :type "PrimitiveComponent Object Reference") (OtherBodyIndex :type Integer) (bFromSweep :type Boolean) (SweepResult :type "HitResult Structure (by ref)"))
  (`KismetSystemLibrary.PrintString` (`KismetSystemLibrary.GetDisplayName` OtherActor))
  (bind _asbp_road_center (cast `/Game/MyBPs/Control/BP_RoadCenter` OtherActor)
    (:`then`
      (`/Game/MyBPs/Control/BP_ControlRoadCenter.ReSpawnActor` (`self.BP_ControlRoadRef_Center`) _asbp_road_center))
    (:`CastFailed`
      (bind _asbp_road_left (cast `/Game/MyBPs/Control/BP_RoadLeft` OtherActor)
        (:`then`
          (`/Game/MyBPs/Control/BP_ControlRoadLeft.ReSpawnActor` (`self.BP_ControlRoadRef_Left`) _asbp_road_left))
        (:`CastFailed`
          (bind _asbp_road_right (cast `/Game/MyBPs/Control/BP_RoadRight` OtherActor))
          (`/Game/MyBPs/Control/BP_ControlRoadRight.ReSpawnActor` (`self.BP_ControlRoadRef_Right`) _asbp_road_right))))))

(fn `UserConstructionScript`
  (bind (_boxextent_x _boxextent_y _boxextent_z) (`KismetMathLibrary.BreakVector` (`BoxComponent.BoxExtent` (`self.BoxCollision`))))
  (`BoxComponent.SetBoxExtent` (`self.BoxCollision`) (`KismetMathLibrary.MakeVector` _boxextent_x (`self.BoxCollisionHeight`) _boxextent_z) true))