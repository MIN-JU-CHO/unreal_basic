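; BP_RoadLeft is a road actor, apparently the left-side piece, that decorates itself with ten randomized building components.
; All work runs in the Construction Script, which loops over the components to randomize footprint, height and X/Y position at a fixed Z.
; Each gets a material from MatArray, though the random index range is pinned to one entry.
; The event graph holds only disabled default events.
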(fn `UserConstructionScript`
  (`parent.UserConstructionScript`)
  (bind _output_get (set `self.BuildingArray` (`|MakeArray` (`self.Build1`) (`self.Build2`) (`self.Build3`) (`self.Build4`) (`self.Build5`) (`self.Build6`) (`self.Build7`) (`self.Build8`) (`self.Build9`) (`self.Build10`))))
  (for _array_element _output_get
    (`SceneComponent.SetRelativeScale3D` _array_element (`KismetMathLibrary.MakeVector` (`KismetMathLibrary.RandomFloatInRange` 0.1 0.2) (`KismetMathLibrary.RandomFloatInRange` 0.1 0.2) (`KismetMathLibrary.RandomFloatInRange` 1.0 5.0)))
    (`SceneComponent.K2_SetRelativeLocation` _array_element (`KismetMathLibrary.MakeVector` (`KismetMathLibrary.RandomFloatInRange` -40.0 40.0) (`KismetMathLibrary.RandomFloatInRange` -40.0 17.0) 100.0) false false)
    (`PrimitiveComponent.SetMaterial` _array_element 0 (`|GetArrayItem` (`self.MatArray`) (`KismetMathLibrary.RandomIntegerInRange` 2 2)))))