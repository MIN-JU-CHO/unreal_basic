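; BP_MoveComponent is an actor component that moves its owning actor at a speed set by the GameManager.
; On BeginPlay it finds and caches the GameManager through a Blueprint library lookup.
; Each Tick it adds a local offset built from the owner's forward vector, GameManager's MoveDelta and delta seconds, without sweep, so the world-space forward vector is applied in local space.
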(event `self.ReceiveBeginPlay`
  ;[1 1 1] 처음에 GameManager 찾는다
  (bind (_gamemanager _isvalid) (`/Game/MyBPs/BPL_GetGameManagerRef.BPL Get Game Manager Ref`))
  (if _isvalid
    (set `self.GameManagerRef` _gamemanager)))

(event `self.ReceiveTick`
  (params (DeltaSeconds :type "Float (single-precision)"))
  (bind _returnvalue (`self.GetOwner`))
  (set `self.DeltaSecond` DeltaSeconds)
  (`Actor.K2_AddActorLocalOffset` _returnvalue (* (* (`Actor.GetActorForwardVector` _returnvalue) (`/Game/MyBPs/BP_GameManager.MoveDelta` (`self.GameManagerRef`))) (`self.DeltaSecond`)) false false))