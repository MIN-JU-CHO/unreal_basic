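; Rot_BP is an actor that moves its Cube along world Y every tick and rotates itself locally while IsRot is set.
; CallEventRot sets that flag and tells the referenced Patrol BP to toggle its patrol via CallStopPatrol with the inverted value.
; On BeginPlay it fires an event dispatcher twice with numeric codes after delays, commented as class-to-level communication.
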(event `self.ReceiveBeginPlay`
  ;[1 1 1] class->level 통신
  ; input number :1000->999
  (`KismetSystemLibrary.Delay` 2.0)
  (`self.EventDispatcher_EventBP` 100)
  (`KismetSystemLibrary.Delay` 2.0)
  (`self.EventDispatcher_EventBP` 999))

(event `CallEventRot`
  (params (IsRot :type Boolean))
  ;[1 1 1] class->class (communication)
  ;;[1 1 1] level->class (communication)
  (bind _output_get (set `self.IsRot` IsRot))
  (if _output_get
    (`/Game/MyBPS/Patrol_BP.CallStopPatrol` (`self.referencePatrolBP`) false)
    (else
      (`/Game/MyBPS/Patrol_BP.CallStopPatrol` (`self.referencePatrolBP`) true))))

(event `self.ReceiveTick`
  (params (DeltaSeconds :type "Float (single-precision)"))
  ;[1 1 1] target 확인 (Actor인지 Component인지)
  ; world와 local 둘의 구분이 필요
  ;;[1 1 1] move
  (`SceneComponent.K2_AddWorldOffset` (`self.Cube`) (0.0 2.0 0.0) false false)
  (if (`self.IsRot`)
    ;;[1 1 1] rotate
    (`self.K2_AddActorLocalRotation` (struct :`Roll` 2.0))))

(fn `UserConstructionScript`)