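; Left_BP is an actor Blueprint that slides itself along negative Y when its col_L event is called with a true flag.
; The event loops through a short Delay, applying a one-unit unswept local offset per step until a counter passes 100.
; It then clears the flag and resets the counter for the next trigger.
; BeginPlay, overlap, Tick and the construction script are empty.
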(event `col_L`
  (params (setstop :type Boolean))
  ;[1 1 1] 충돌 시 마다 반복문 실행
  (bind _output_get (set `self.isstop` setstop))
  (if _output_get :!label _label
    (`self.K2_AddActorLocalOffset` (0.0 -1.0 0.0))
    ;[1 1 1] 자연스러운 움직임
    (`KismetSystemLibrary.Delay` 0.01)
    ;[1 1 1] for
    (`/Engine/EditorBlueprintResources/StandardMacros.IncrementInt` (`self.loopss`)
      (:`  `
        (if (<= (`self.loopss`) 100)
          (goto _label)
          (else
            ;[1 1 1] loop 빠져 나올 때 처리
            (set `self.isstop` false)
            (set `self.loopss` 0)))))))

(fn `UserConstructionScript`)