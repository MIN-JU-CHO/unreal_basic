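; LTriggerBox_BP is a Blueprint that nudges its Cone component in small steps through the custom event col_L.
; When Isstop is true, col_L offsets the Cone along negative X without sweep, increments Lops, and clears Isstop while the count stays within a small limit.
; Nothing here calls col_L or sets Isstop true; overlap, BeginPlay and Tick are empty, and a node hiding the Cone is disconnected.
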(event `col_L`
  (if (`self.isstop`)
    (`SceneComponent.K2_AddWorldOffset` (`self.Cone`) (-2.0 0.0 0.0) false false)
    (`/Engine/EditorBlueprintResources/StandardMacros.IncrementInt` (`self.lops`)
      (:`  `
        (if (<= (`self.lops`) 9)
          (set `self.isstop` false))))))

(event `self.ReceiveBeginPlay`)

(fn `UserConstructionScript`)