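; Patrol actor Blueprint that moves its Cube component back and forth along the world Y axis.
; Each Tick, while the patrol flag is on, it offsets the Cube by a fixed per-frame step, flipping direction at fixed world-space bounds either side of zero.
; The CallStopPatrol event lets other classes set that flag.
; An alternative version using actor location is left disconnected.
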(event `CallStopPatrol`
  (params (IsPatrol :type Boolean))
  ;[1 1 1] Patrol 여부 통신(class->class)
  (set `self.Ispatrol` IsPatrol))

(event `self.ReceiveBeginPlay`
  ;[1 1 1] world location 이용
  (set `self.W_loc` (`SceneComponent.K2_GetComponentLocation` (`self.Cube`))))

(event `self.ReceiveTick`
  (params (DeltaSeconds :type "Float (single-precision)"))
  (bind (_returnvalue_x _returnvalue_y) (`KismetMathLibrary.BreakVector` (`SceneComponent.K2_GetComponentLocation` (`self.Cube`))))
  (bind (_returnvalue_x_2 _returnvalue_y_2) (`KismetMathLibrary.BreakVector` (`SceneComponent.K2_GetComponentLocation` (`self.Cube`))))
  ;[1 1 1] Patrol 여부 먼저 확인 후
  (if (`self.Ispatrol`)
    ;[1 1 1] world location 이용
    (if (`self.isturn`)
      (`SceneComponent.K2_AddWorldOffset` (`self.Cube`) (0.0 2.0 0.0) false false)
      (if (>= _returnvalue_y_2 350.0)
        (set `self.isturn` false))
      (else
        (`SceneComponent.K2_AddWorldOffset` (`self.Cube`) (0.0 -2.0 0.0) false false)
        (if (<= _returnvalue_y -350.0)
          (set `self.isturn` true))))))

(fn `UserConstructionScript`)